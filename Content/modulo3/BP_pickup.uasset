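; Pickup actor that spins and bobs in place until something overlaps its box.
; BeginPlay starts an endless short-Delay loop, used instead of Tick, that rotates the static mesh and moves it up and down, flipping direction at height limits relative to its starting Z.
; Any box overlap destroys the actor and spawns an explosion particle at its location, with no check on what overlapped.
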(event `self.ReceiveBeginPlay`
  (bind _initial_z (`self.Initial Z`))
  (bind _staticmesh (`self.StaticMesh`))
  (bind (_relativelocation_x _relativelocation_y _relativelocation_z) (`KismetMathLibrary.BreakVector` (`SceneComponent.RelativeLocation` (`self.StaticMesh`))))
  (bind (_relativelocation_x_2 _relativelocation_y_2 _relativelocation_z_2) (`KismetMathLibrary.BreakVector` (`SceneComponent.RelativeLocation` _staticmesh)))
  (set `self.delta` 50.0)
  (set `self.Initial Z` _relativelocation_z)
  (set `self.isUp` true)
  (`SceneComponent.K2_AddLocalRotation` (`self.StaticMesh`) (struct :`Yaw` 1.0) false false :!label _label)
  (if (`self.isUp`)
    (`SceneComponent.K2_AddLocalOffset` _staticmesh (0.0 0.0 1.0) false false)
    (set `self.isUp` (not (>= _relativelocation_z_2 (+ _initial_z 75.0))))
    (else
      (`SceneComponent.K2_AddLocalOffset` _staticmesh (0.0 0.0 -1.0) false false)
      (set `self.isUp` (<= _relativelocation_z_2 (+ _initial_z -25.0)))))
  (`KismetSystemLibrary.Delay` 0.01)
  (goto _label))

(event `self.Box.OnComponentBeginOverlap`
  (params (OverlappedComponent :type "PrimitiveComponent Object Reference") (OtherActor :type "Actor Object Reference") (OtherComp :type "PrimitiveComponent Object Reference") (OtherBodyIndex :type Integer) (bFromSweep :type Boolean) (SweepResult :type "HitResult Structure (by ref)"))
  (`self.K2_DestroyActor`)
  (`GameplayStatics.SpawnEmitterAtLocation` "/Game/StarterContent/Particles/P_Explosion.P_Explosion" (`self.K2_GetActorLocation`)))

(fn `UserConstructionScript`)